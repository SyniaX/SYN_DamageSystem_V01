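; Ability component for the SYN ability system that manages a character's learned abilities, levels, slot bindings, cooldowns and main target.
; Abilities are objects built from DB_AbilityInfo rows on authority, tracked alongside an ID-to-level map.
; SERVER events wrap changes and execution, with bound slots resolving to IDs before the execute call.
; Cooldowns are stored as game-time end stamps, and a forward trace from player 0 selects actors tagged Targetable.
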(event `INIT SYN Ability Component`
  (params (`Character Skeleton` :type "SkeletalMeshComponent Object Reference") (`Weapon Mesh` :type "SkeletalMeshComponent Object Reference"))
  ;[0 0.7254 1] INIT Ability Component // Only Needed when you want to Execute Montages
  (set `self.Owner Character Mesh` `Character Skeleton`)
  (set `self.Owner Weapon Mesh` `Weapon Mesh`))

(event `SERVER // Add Ability`
  (params (ID :type Name) (Level :type Integer))
  ;[1 0 0.1564] SERVER // Add Ability
  (`self.Add Ability` ID Level))

(event `SERVER // Update Ability Cooldown`
  (params (`Ability ID` :type "Name (by ref)") (Cooldown :type "Float (double-precision)"))
  ;[1 0 0.1564] SERVER // Update Ability Cooldown
  (`self.Update Ability Cooldown` `Ability ID` Cooldown))

(event `SERVER // Clear Abilities`
  ;[1 0 0.1564] SERVER // Clear Abilities
  (`self.Clear Abilities`))

(event `SERVER // Change Main Target`
  (params (`New Main Target` :type "Actor Object Reference"))
  ;[1 0 0.1564] SERVER // Change Main Target
  (set `self.Selected Main Target` `New Main Target`))

(event `SERVER // Remove Ability`
  (params (Key :type "Name (by ref)"))
  ;[1 0 0.1564] SERVER // Remove Ability
  (`self.Remove Ability` Key))

(event `SERVER // Execute Ability`
  (params (ID :type Name))
  ;[1 0 0.1564] SERVER // Execute Ability
  (`self.Execute Ability` ID))

(event `SERVER // Change Ability Level`
  (params (ID :type Name) (Level :type Integer))
  ;[1 0 0.1564] SERVER // Change Ability Level
  (`self.Change Ability Level` ID Level))

(event `SERVER // Update Global Cooldown`
  (params (`Global Cooldown` :type "Float (double-precision)"))
  ;[1 0 0.1564] SERVER // Update Global Cooldown
  (`self.Execute Global Cooldown` `Global Cooldown`))

(event `SERVER // Load Ability Set`
  (params (Abilities :type "Map of Name to Integer"))
  ;[1 0 0.1564] SERVER // Load Ability Set
  (`self.Load Ability Set` Abilities))

(fn `Add Ability`
  (params (ID :type Name) (Level :type Integer))
  ;[1 1 1] Add Ability // Authority Only
  (`self.Owner Has Authority`
    (:`true`
      (bind (_array_element _success) (`self.Find Ability` ID))
      (if _success
        (`KismetSystemLibrary.PrintString` "Ability exists // Try to Modify")
        (else
          (`BlueprintMapLibrary.Map_Add` (`self.Learned Abilities`) ID Level)
          (`self.Construct Ability` (`Pawn.GetController` (cast `Pawn` (`self.GetOwner`) :!pure true)) ID Level))))))

(fn `Bind Ability`
  (params (Slot :type "/Game/SYN/AbilitySystem/Enumeration/E_AbilitySlots Enum" :default "NewEnumerator0") (`Ability ID` :type Name))
  (`BlueprintMapLibrary.Map_Add` (`self.Ability Bindings`) Slot `Ability ID`))

(fn `Change Ability Level`
  (params (ID :type "Name (by ref)") (Level :type "Integer (by ref)"))
  (bind _learned_abilities (`self.Learned Abilities`))
  (if (`BlueprintMapLibrary.Map_Contains` _learned_abilities ID)
    (`BlueprintMapLibrary.Map_Add` _learned_abilities ID Level)
    (bind (_array_element _success) (`self.Find Ability` ID))
    (if _success
      (set `/Game/SYN/AbilitySystem/Blueprints/Abilities/U_Ability.Level` Level _array_element)
      (`self.On Change Ability Level` ID Level))))

(fn `Clear Abilities`
  (returns (ReturnValue :type Boolean))
  (`BlueprintMapLibrary.Map_Clear` (`self.Learned Abilities`))
  (`KismetArrayLibrary.Array_Clear` (`self.Ability Array`))
  (`self.On Clear Abilities`)
  (return true))

(fn `Construct Ability`
  (params (`Owning Controller` :type "Controller Object Reference") (ID :type Name) (Level :type Integer))
  (returns (Ability :type "/Game/SYN/AbilitySystem/Blueprints/Abilities/U_Ability Object Reference"))
  (bind _returnvalue (`|GetDataTableRow` "/Game/SYN/AbilitySystem/DataTables/DB_AbilityInfo.DB_AbilityInfo" ID)
    (:`then`
      (bind _returnvalue_2 (`|GenericCreateObject` (`.AbilityClass_11_4EF348374DB6C3311EE82BBDEF29F0ED` (break `/Game/SYN/AbilitySystem/Structures/S_AbilityInfo` _returnvalue)) self `Owning Controller` self ID Level _returnvalue))
      (`KismetArrayLibrary.Array_Add` (`self.Ability Array`) _returnvalue_2)
      (return _returnvalue_2))))

(fn `Execute Ability`
  (params (ID :type Name))
  (returns (Success :type Boolean))
  (if (`.ReturnValue` (`BlueprintMapLibrary.Map_Find` (`self.Learned Abilities`) ID))
    (bind (_array_element _success) (`self.Find Ability` ID))
    (if _success
      (`/Game/SYN/AbilitySystem/Blueprints/Abilities/U_Ability.Execute Ability` _array_element))
    (else
      (return false))))

(fn `Execute Global Cooldown`
  (params (`Global Cooldown` :type "Float (double-precision)"))
  (bind _output_get (set `self.Global Cooldown End Time` (+ `Global Cooldown` (`KismetSystemLibrary.GetGameTimeInSeconds`))))
  (`self.On Update Global Cooldown` _output_get))

(fn `Find Ability`
  (params (ID :type Name))
  (returns (`Array Element` :type "/Game/SYN/AbilitySystem/Blueprints/Abilities/U_Ability Object Reference") (Success :type Boolean))
  (bind _returnvalue (`BlueprintMapLibrary.Map_Contains` (`self.Learned Abilities`) ID))
  (for _array_element (`self.Ability Array`)
    (if (and (== (`/Game/SYN/AbilitySystem/Blueprints/Abilities/U_Ability.Get ID` _array_element) ID) _returnvalue)
      (return _array_element true)
      (elif (not _returnvalue)
        (`KismetSystemLibrary.PrintString` "ERROR // Ability exists but it isnt Learned")
        (return null false))))
  (return null false))

(fn `Find Target and Set Main Target`
  (bind _returnvalue (`GameplayStatics.GetPlayerPawn` 0))
  (bind (_outhit _returnvalue_2) (`self.Trace Forward` (+ (`Actor.K2_GetActorLocation` _returnvalue) (`KismetMathLibrary.MakeVector` 0.0 0.0 (`Pawn.BaseEyeHeight` _returnvalue))) (`Pawn.GetBaseAimRotation` _returnvalue) 10000.0 "TraceTypeQuery1" (`|MakeArray` _returnvalue :!type "Actor Object Reference")))
  (if _returnvalue_2
    (bind (_bblockinghit _binitialoverlap _time _distance _location _impactpoint _normal _impactnormal _physmat _hitactor) (`GameplayStatics.BreakHitResult` _outhit))
    (if (`Actor.ActorHasTag` _hitactor "Targetable")
      (`self.SERVER // Change Main Target` _hitactor))))

(fn `Is Ability On Cooldown?`
  (params (`Ability ID` :type "Name (by ref)"))
  (returns (ReturnValue :type Boolean))
  (bind (_value _returnvalue) (`BlueprintMapLibrary.Map_Find` (`self.Ability Cooldowns`) `Ability ID`))
  (return (and _returnvalue (> _value (`KismetSystemLibrary.GetGameTimeInSeconds`)))))

(fn `Is Global Cooldown Active?`
  (returns (ReturnValue :type Boolean))
  (return (> (`self.Global Cooldown End Time`) (`KismetSystemLibrary.GetGameTimeInSeconds`))))

(fn `Load Ability Mapping Set`
  (params (Slots :type "Map of /Game/SYN/AbilitySystem/Enumeration/E_AbilitySlots Enum to Name" :default _))
  (bind _keys (`BlueprintMapLibrary.Map_Keys` Slots))
  (for _array_element _keys
    (`self.Bind Ability` _array_element (`BlueprintMapLibrary.Map_Find` Slots _array_element))))

(fn `Load Ability Set`
  (params (Abilities :type "Map of Name to Integer"))
  (`self.Owner Has Authority`
    (:`true`
      (`self.Clear Abilities`)
      (bind _keys (`BlueprintMapLibrary.Map_Keys` Abilities))
      (for _array_element _keys
        (`self.Add Ability` _array_element (`BlueprintMapLibrary.Map_Find` Abilities _array_element))))))

(fn `Remove Ability`
  (params (Key :type "Name (by ref)"))
  (returns (ReturnValue :type Boolean))
  (bind _returnvalue (`BlueprintMapLibrary.Map_Remove` (`self.Learned Abilities`) Key))
  (for (_array_element _array_index) (`self.Ability Array`)
    (if (== (`/Game/SYN/AbilitySystem/Blueprints/Abilities/U_Ability.Get ID` _array_element) Key)
      (`KismetArrayLibrary.Array_Remove` (`self.Ability Array`) _array_index)
      (`self.On Remove Ability` Key)))
  (return _returnvalue))

(fn `Remove Ability Binding`
  (params (Slot :type "/Game/SYN/AbilitySystem/Enumeration/E_AbilitySlots Enum" :default "NewEnumerator0"))
  (`BlueprintMapLibrary.Map_Remove` (`self.Ability Bindings`) Slot))

(fn `Spawn Actor`
  (params (Class :type "Actor Class Reference") (SpawnTransform :type "Transform Structure") (CollisionHandlingOverride :type "ESpawnActorCollisionHandlingMethod Enum" :default "Undefined") (Owner :type "Actor Object Reference") (Instigator :type "Pawn Object Reference"))
  (returns (ReturnValue :type "Actor Object Reference"))
  (bind _returnvalue (`|SpawnActorFromClass` Class SpawnTransform CollisionHandlingOverride "OverrideRootScale" Owner Instigator))
  (return _returnvalue))

(fn `Trace Forward`
  (params (`Start Vector` :type "Vector Structure") (Direction :type "Rotator Structure") (Length :type "Float (double-precision)") (`Trace Channel` :type "ETraceTypeQuery Enum" :default "TraceTypeQuery1") (`Actors to Ignore` :type "Array of Actor Object Reference (by ref)"))
  (returns (OutHit :type "HitResult Structure") (ReturnValue :type Boolean))
  (bind (_outhit _returnvalue) (`KismetSystemLibrary.LineTraceSingle` `Start Vector` (+ `Start Vector` (* (`KismetMathLibrary.GetForwardVector` Direction) Length)) `Trace Channel` false `Actors to Ignore` "ForDuration" true (struct :`R` 1.0 :`B` 0.965993 :`A` 1.0) (struct :`R` 0.060262 :`G` 1.0 :`A` 1.0)))
  (return _outhit _returnvalue))

(fn `Try to Execute Ability Slot`
  (params (Slot :type "/Game/SYN/AbilitySystem/Enumeration/E_AbilitySlots Enum" :default "NewEnumerator0"))
  (bind (_value _returnvalue) (`BlueprintMapLibrary.Map_Find` (`self.Ability Bindings`) Slot))
  (if _returnvalue
    (`self.SERVER // Execute Ability` _value)
    (else
      (`KismetSystemLibrary.PrintString` "Not Found"))))

(fn `Update Ability Cooldown`
  (params (`Ability ID` :type "Name (by ref)") (Cooldown :type "Float (double-precision) (by ref)"))
  (bind _returnvalue (+ Cooldown (`KismetSystemLibrary.GetGameTimeInSeconds`)))
  (`BlueprintMapLibrary.Map_Add` (`self.Ability Cooldowns`) `Ability ID` _returnvalue)
  (`self.On Update Ability Cooldown` `Ability ID` _returnvalue))