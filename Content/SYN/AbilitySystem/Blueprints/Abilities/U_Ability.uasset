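; Base ability object whose ExecuteAbility event, meant for authority only, runs an ability if neither its own nor the global cooldown is active.
; It sets cooldowns through the owner's ability component as AbilityInfo flags allow, calls the empty OnExecuteAbility hook, then plays any valid montage on the owner's mesh.
; Helpers read per-level value arrays at Level minus one, falling back to the last entry when out of range.
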(event `Execute Ability`
  (bind _returnvalue (`self.Try to get Ability Component from Owner`))
  (bind ((`Montage_41_8FCADE7C44FDCB1587EF36AC03117A68` _montage)) (break `/Game/SYN/AbilitySystem/Structures/S_AbilityInfo` (`self.Ability Info`)))
  (bind ((`SetCooldowninParent_44_6E221FBE4C66660A052DEC968E70423B` _setcooldowninparent) (`AbilityCooldown_28_95088CAB4DE960F028B922AA118063DE` _abilitycooldown) (`ExecutesGlobalCooldown_34_9B45B55E4012B28EA43F9D90A143F6AF` _executesglobalcooldown) (`GlobalCooldown_38_F8C576FC4C6054C5C8ADAA8A41239D48` _globalcooldown)) (break `/Game/SYN/AbilitySystem/Structures/S_AbilityInfo` (`self.Ability Info`)))
  ;[1 1 1] Execute Ability // Only Call this from Authority
  (if (and (not (`/Game/SYN/AbilitySystem/Blueprints/C_SYNAbility.Is Global Cooldown Active?` _returnvalue)) (not (`/Game/SYN/AbilitySystem/Blueprints/C_SYNAbility.Is Ability On Cooldown?` _returnvalue (`self.ID`))))
    (`|ExecutionSequence`
      (:`then_0`
        ;[1 1 1] Set Cooldowns
        (if (not _setcooldowninparent)
          (`self.Set Ability Cooldown` (`self.Get Float Value by Level` _abilitycooldown))
          (if _executesglobalcooldown
            (`self.Set Global Cooldown` (`self.Get Float Value by Level` _globalcooldown)))))
      (:`then_1`
        ;[1 1 1] On Execute Ability
        (`self.On Execute Ability`))
      (:`then_2`
        ;[1 1 1] Play Animation Montage when its Valid
        (`/Engine/EditorBlueprintResources/StandardMacros.IsValid` _montage
          (:`Is Valid`
            (`|PlayMontage` (`/Game/SYN/AbilitySystem/Blueprints/C_SYNAbility.Owner Character Mesh` (`self.Try to get Ability Component from Owner`)) _montage)))))
    (else
      (`KismetSystemLibrary.PrintString` null "// Cooldown //" true true (struct :`G` 1.0 :`B` 0.058634 :`A` 1.0)))))

(fn `Get Ability Value`
  (params (Values :type "Array of /Game/SYN/AbilitySystem/Structures/S_AbilityValue Structure") (`Value Index` :type Integer))
  (returns (Output :type "Float (double-precision)") (`Description (Debug)` :type Text))
  (bind (_description _value) (break `/Game/SYN/AbilitySystem/Structures/S_AbilityValue` (`|GetArrayItem` Values `Value Index`)))
  (return (`self.Get Float Value by Level` _value) _description))

(fn `Get Float Value by Level`
  (params (Array :type "Array of Float (double-precision)"))
  (returns (Output :type "Float (double-precision)"))
  (bind _returnvalue (- (`self.Level`) 1))
  (return (`|GetArrayItem` Array (`KismetMathLibrary.SelectInt` _returnvalue (`KismetArrayLibrary.Array_LastIndex` Array) (`KismetArrayLibrary.Array_IsValidIndex` Array _returnvalue)))))

(fn `Get ID`
  (returns (ID :type Name))
  (return (`self.ID`)))

(fn `On Execute Ability`)

(fn `Set Ability Cooldown`
  (params (Cooldown :type "Float (double-precision)"))
  (`/Game/SYN/AbilitySystem/Blueprints/C_SYNAbility.SERVER // Update Ability Cooldown` (`self.Try to get Ability Component from Owner`) (`self.ID`) Cooldown))

(fn `Set Global Cooldown`
  (params (`Global Cooldown` :type "Float (double-precision)"))
  (`/Game/SYN/AbilitySystem/Blueprints/C_SYNAbility.SERVER // Update Global Cooldown` (`self.Try to get Ability Component from Owner`) `Global Cooldown`))