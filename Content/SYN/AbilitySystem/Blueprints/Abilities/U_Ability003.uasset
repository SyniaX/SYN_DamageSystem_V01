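; Multi-target ability that marks "Targetable" actors with forward eye traces, aiming to damage four at once.
; First use opens a timed window via DoOnce; each use adds a hit, and a use with three marks traces again, damages all and starts cooldown.
; Timeout resets DoOnce, clears marks and applies half cooldown.
; The damage path cancels the timer without closing the window, clearing marks only with global cooldown.
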(event `self.On Execute Ability`
  (bind _ability_owner (`self.Ability Owner`))
  (bind _ability_owner_2 (`self.Ability Owner`))
  (bind ((`AbilityCooldown_28_95088CAB4DE960F028B922AA118063DE` _abilitycooldown) (`ExecutesGlobalCooldown_34_9B45B55E4012B28EA43F9D90A143F6AF` _executesglobalcooldown) (`GlobalCooldown_38_F8C576FC4C6054C5C8ADAA8A41239D48` _globalcooldown)) (break `/Game/SYN/AbilitySystem/Structures/S_AbilityInfo` (`self.Ability Info`)))
  (bind (_outlocation _outrotation) (`Actor.GetActorEyesViewPoint` _ability_owner))
  (`|ExecutionSequence`
    (:`then_0`
      (`/Engine/EditorBlueprintResources/StandardMacros.DoOnce` false :!label _label
        (:`Completed`
          (bind _returnvalue (`KismetSystemLibrary.K2_SetTimerDelegate` (delegate `Close Target Window`) 10.0))
          (set `self.Target Window is Open` true)
          (`KismetSystemLibrary.PrintString` null "Open Window"))))
    (:`then_1`
      (if (`self.Target Window is Open`)
        (if (== (`BlueprintSetLibrary.Set_Length` (`self.Marked Targets`)) 3)
          (`|ExecutionSequence`
            (:`then_0`
              ;[1 1 1] Try to Find Target
              (bind (_outhit _returnvalue_2) (`/Game/SYN/AbilitySystem/Blueprints/C_SYNAbility.Trace Forward` (`self.Ability Component`) _outlocation _outrotation 10000.0 "TraceTypeQuery1" (`|MakeArray` (`Controller.K2_GetPawn` _ability_owner) :!type "Actor Object Reference") :!label _label_2))
              (if _returnvalue_2
                (bind (_bblockinghit _binitialoverlap _time _distance _location _impactpoint _normal _impactnormal _physmat _hitactor) (`GameplayStatics.BreakHitResult` _outhit))
                (if (`Actor.ActorHasTag` _hitactor "Targetable")
                  (`BlueprintSetLibrary.Set_Add` (`self.Marked Targets`) _hitactor))))
            (:`then_1`
              ;[1 1 1] On Reach 4 Targets
              (`KismetSystemLibrary.K2_InvalidateTimerHandle` _returnvalue)
              (bind _result (`BlueprintSetLibrary.Set_ToArray` (`self.Marked Targets`)))
              (for _array_element _result
                (`GameplayStatics.ApplyDamage` _array_element (`self.Get Ability Value` (`.Values_32_625928D74386AFB5625DB9BFD679DD5D` (break `/Game/SYN/AbilitySystem/Structures/S_AbilityInfo` (`self.Ability Info`)))) _ability_owner_2 (`Controller.K2_GetPawn` _ability_owner_2) "/Game/SYN/DamageSystem/Blueprints/DamageTypes/DT_SYNDamageType.DT_SYNDamageType_C"))
              (`self.Set Ability Cooldown` (`self.Get Float Value by Level` _abilitycooldown))
              (if _executesglobalcooldown
                (`self.Set Global Cooldown` (`self.Get Float Value by Level` _globalcooldown))
                (`BlueprintSetLibrary.Set_Clear` (`self.Marked Targets`)))))
          (else
            (goto _label_2)))))))

(event `Close Target Window`
  ;[1 1 1] Doesnt Reach 4 Targets // Reset Ability and apply 1/2 Cooldown
  (`|ExecutionSequence`
    (:`then_0`
      (goto _label :!via `Reset`))
    (:`then_1`
      (set `self.Target Window is Open` false)
      (`self.Set Ability Cooldown` (/ (`self.Get Float Value by Level` (`.AbilityCooldown_28_95088CAB4DE960F028B922AA118063DE` (break `/Game/SYN/AbilitySystem/Structures/S_AbilityInfo` (`self.Ability Info`)))) 2.0))
      (`BlueprintSetLibrary.Set_Clear` (`self.Marked Targets`)))))