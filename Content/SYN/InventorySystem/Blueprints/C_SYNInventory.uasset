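; Inventory component that stores items in a slot array and handles setting, moving and stacking them.
; SERVER-labelled events initialise the slot count, set items and move items, delegating to helper functions for resizing, slot lookup and counting.
; MoveItem works within or across inventories, sending matching stackable items with free space to AddItemAmount and other cases to a swap branch.
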(event `SERVER // INIT Inventory`
  (params (`Inventory Slots` :type Integer))
  ;[1 1 1] SERVER // INIT Inventory
  (`self.Clear Inventory`)
  (`self.Increase Inventory Size` `Inventory Slots`))

(event `SERVER // Move Item`
  (params (`Source Inventory` :type "/Game/SYN/InventorySystem/Blueprints/C_SYNInventory Object Reference") (`Source Slot` :type Integer) (`Target Slot` :type Integer))
  ;[1 1 1] SERVER // INIT Inventory
  (`self.Move Item` `Source Inventory` `Source Slot` `Target Slot`))

(event `SERVER // Set Item`
  (params (Slot :type Integer) (Item1 :type "/Game/SYN/InventorySystem/Sturctures/S_Item Structure"))
  ;[1 1 1] SERVER // Set Item
  (`self.Set Inventory Item` Slot Item1))

(fn `Add Item Amount`
  (params (Slot :type Integer) (Amount :type Integer))
  (returns (`Remaining Amount` :type Integer))
  (locals (`Item to add Amount` :type " Structure") (`Local Amount` :type Integer) (`Local Target Stack Space` :type Integer) (`Item to Add` :type "/Game/SYN/InventorySystem/Sturctures/S_Item Structure"))
  (bind _item_to_add (`local.Item to Add`))
  (bind _output_get (set `local.Item to Add` (`|GetArrayItem` (`self.Inventory`) Slot)))
  (set `local.Local Amount` Amount)
  (bind _returnvalue (`/Game/SYN/InventorySystem/Blueprints/BP_InventoryMacroLibrary.Get Stack Space` _output_get))
  (bind _output_get_2 (set `local.Local Target Stack Space` _returnvalue))
  (if (> _returnvalue 0)
    (if (> (`local.Local Amount`) (`local.Local Target Stack Space`))
      (bind _structout (setmembers `/Game/SYN/InventorySystem/Sturctures/S_Item` :`StructRef` _item_to_add :`Stack Amount` (`/Game/SYN/InventorySystem/Blueprints/BP_InventoryMacroLibrary.Get Max Stack Size` _item_to_add)))
      (`self.Set Inventory Item` Slot _structout)
      (return (- (`local.Local Amount`) (`local.Local Target Stack Space`)))
      (else
        (bind _structout_2 (setmembers `/Game/SYN/InventorySystem/Sturctures/S_Item` :`StructRef` (`local.Item to Add`) :`Stack Amount` 0))
        (`self.Set Inventory Item` Slot _structout_2)
        (return 0)))
    (else
      (return _output_get_2))))

(fn `Clear Inventory`
  (`KismetArrayLibrary.Array_Clear` (`self.Inventory`)))

(fn `Decrease Inventory Size`
  (params (Amount :type Integer))
  (returns (Success :type Boolean))
  (bind _inventory (`self.Inventory`))
  (for _ (range 1 (+ Amount 1))
    (`KismetArrayLibrary.Array_Remove` _inventory (`KismetArrayLibrary.Array_LastIndex` _inventory)))
  (return true))

(fn `Get Empty Inventory Slot`
  (returns (`Empty Slot` :type Integer) (Success :type Boolean))
  (locals (`Local Empty Slot` :type Integer) (`Local Success` :type Boolean))
  (for (_array_element _array_index) (`self.Inventory`)
    (`/Game/SYN/InventorySystem/Blueprints/BP_InventoryMacroLibrary.Is Valid Item?` _array_element
      (:`false`
        (`|ExecutionSequence`
          (:`then_0`
            (set `local.Local Empty Slot` _array_index)
            (set `local.Local Success` true))
          (:`then_1`
            (break))))))
  (return (`local.Local Empty Slot`) (`local.Local Success`)))

(fn `Get Inventory Item`
  (params (Slot :type Integer))
  (returns (Item :type "/Game/SYN/InventorySystem/Sturctures/S_Item Structure"))
  (bind _output (`|GetArrayItem` (`self.Inventory`) Slot))
  (`/Game/SYN/InventorySystem/Blueprints/BP_InventoryMacroLibrary.Is Valid Item?` _output
    (:`true`
      (return _output))
    (:`false`
      (return _output))))

(fn `Get Inventory Item Count`
  (returns (`Item Counter` :type Integer))
  (locals (`Local Item Counter` :type Integer))
  (for _array_element (`self.Inventory`)
    (`/Game/SYN/InventorySystem/Blueprints/BP_InventoryMacroLibrary.Is Valid Item?` _array_element
      (:`true`
        (`/Engine/EditorBlueprintResources/StandardMacros.IncrementInt` (`local.Local Item Counter`)))))
  (return (`local.Local Item Counter`)))

(fn `Increase Inventory Size`
  (params (`Inventory Slots` :type Integer))
  (returns (Success :type Boolean))
  (for _ (range 1 (+ `Inventory Slots` 1))
    (`KismetArrayLibrary.Array_Add` (`self.Inventory`)))
  (return true))

(fn `Move Item`
  (params (`Source Inventory` :type "/Game/SYN/InventorySystem/Blueprints/C_SYNInventory Object Reference") (`Source Slot` :type Integer :default 0) (`Target Slot` :type Integer))
  (locals (`Local Source Inventory` :type "/Game/SYN/InventorySystem/Blueprints/C_SYNInventory Object Reference") (`Local Source Slot` :type Integer) (`Local Target Slot` :type Integer) (`Local Target Item` :type "/Game/SYN/InventorySystem/Sturctures/S_Item Structure") (`Local Source Item` :type "/Game/SYN/InventorySystem/Sturctures/S_Item Structure"))
  (if (and (== `Source Inventory` self) (== `Source Slot` `Target Slot`))
    (`KismetSystemLibrary.PrintString` "Moving Item to Same Slot")
    (else
      (`|ExecutionSequence`
        (:`then_0`
          (set `local.Local Source Inventory` `Source Inventory`))
        (:`then_1`
          (set `local.Local Source Slot` `Source Slot`))
        (:`then_2`
          (set `local.Local Target Slot` `Target Slot`))
        (:`then_3`
          (set `local.Local Source Item` (`|GetArrayItem` (`/Game/SYN/InventorySystem/Blueprints/C_SYNInventory.Inventory` (`local.Local Source Inventory`)) (`local.Local Source Slot`)))
          (bind _output_get (set `local.Local Target Item` (`|GetArrayItem` (`self.Inventory`) (`local.Local Target Slot`))))
          (`/Game/SYN/InventorySystem/Blueprints/BP_InventoryMacroLibrary.Is Valid Item?` _output_get
            (:`true`
              (if (and (`/Game/SYN/InventorySystem/Blueprints/BP_InventoryMacroLibrary.Is Same Item` (`local.Local Source Item`) _output_get) (`/Game/SYN/InventorySystem/Blueprints/BP_InventoryMacroLibrary.Is Stackable` _output_get) (> (`/Game/SYN/InventorySystem/Blueprints/BP_InventoryMacroLibrary.Get Stack Space` _output_get) 0))
                ;[1 1 1] Add Item Amount
                (bind _remaining_amount (`self.Add Item Amount` (`local.Local Target Slot`) (`/Game/SYN/InventorySystem/Blueprints/BP_InventoryMacroLibrary.Get Item Amount` (`local.Local Target Item`))))
                (if (> _remaining_amount 0)
                  (bind _structout (setmembers `/Game/SYN/InventorySystem/Sturctures/S_Item` :`StructRef` (`local.Local Target Item`) :`Stack Amount` _remaining_amount))
                  (`self.Set Inventory Item` (`local.Local Source Inventory`) (`local.Local Source Slot`) _structout)
                  (return)
                  (else
                    (`self.Remove Inventory Item` (`local.Local Source Inventory`) (`local.Local Source Slot`))))
                (else
                  ;[1 1 1] Swap Items
                  (`self.Set Inventory Item` (`local.Local Target Slot`) :!label _label)
                  (`self.Set Inventory Item` :`self` (`local.Local Source Inventory`) :`InventorySlot` (`local.Local Source Slot`))
                  (return))))
            (:`false`
              (goto _label))))))))

(fn `Remove Inventory Item`
  (params (Slot :type Integer))
  (returns (Success :type Boolean))
  (`KismetArrayLibrary.Array_Set` (`self.Inventory`) Slot)
  (return true))

(fn `Set Inventory Item`
  (params (InventorySlot :type Integer) (Item1 :type "/Game/SYN/InventorySystem/Sturctures/S_Item Structure"))
  (returns (Success :type Boolean))
  (if (<= InventorySlot (`KismetArrayLibrary.Array_Length` (`self.Inventory`)))
    (`KismetArrayLibrary.Array_Set` (`self.Inventory`) InventorySlot Item1)
    (return true)
    (else
      (return false))))