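; Player inventory Blueprint that extends a parent inventory and stores equipment and carried items in one array.
; Server init clears it and sizes it to the requested slots plus one per equipment enum entry, reserving the first indices for equipment.
; GetEquipement returns that leading range, while the empty-slot search skips it.
; SetInventoryItem calls the parent, then only prints a stat-update placeholder for equipment indices below the last one.
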(event `self.SERVER // INIT Inventory`
  (params (`Inventory Slots` :type Integer))
  (`self.Clear Inventory`)
  (`self.Increase Inventory Size` (+ `Inventory Slots` (enumcount `/Game/SYN/InventorySystem/Enumerations/E_EquipementSlots`))))

(fn `Get Empty Inventory Slot`
  (returns (`Empty Slot` :type Integer) (Success :type Boolean))
  (locals (`Local Empty Slot` :type Integer) (`Local Success` :type Boolean))
  (for (_array_element _array_index) (`self.Inventory`)
    (`/Game/SYN/InventorySystem/Blueprints/BP_InventoryMacroLibrary.Is Valid Item?` _array_element
      (:`false`
        (if (> _array_index (- (enumcount `/Game/SYN/InventorySystem/Enumerations/E_EquipementSlots`) 1))
          (`|ExecutionSequence`
            (:`then_0`
              (set `local.Local Empty Slot` _array_index)
              (set `local.Local Success` true))
            (:`then_1`
              (break)))))))
  (return (`local.Local Empty Slot`) (`local.Local Success`)))

(fn `Get Equipement`
  (returns (`Local Found1` :type "Array of /Game/SYN/InventorySystem/Sturctures/S_Item Structure"))
  (locals (`Local Found` :type "Array of /Game/SYN/InventorySystem/Sturctures/S_Item Structure"))
  (for _index (range (enumcount `/Game/SYN/InventorySystem/Enumerations/E_EquipementSlots`))
    (`KismetArrayLibrary.Array_Add` (`local.Local Found`) (`|GetArrayItem` (`self.Inventory`) _index)))
  (return (`local.Local Found`)))

(fn `Set Inventory Item`
  (params (InventorySlot :type Integer) (Item1 :type "/Game/SYN/InventorySystem/Sturctures/S_Item Structure"))
  (returns (Success :type Boolean))
  (bind _success (`parent.Set Inventory Item` InventorySlot Item1))
  (if (< InventorySlot (- (enumcount `/Game/SYN/InventorySystem/Enumerations/E_EquipementSlots`) 1))
    (`KismetSystemLibrary.PrintString` "Update Stats")
    (else
      (return _success))))