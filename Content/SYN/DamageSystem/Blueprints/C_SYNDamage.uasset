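; C_SYNDamage is a damage component for the SYN damage system, still a debug stub that intercepts damage taken by its owning actor.
; On BeginPlay it binds to the owner's OnTakeAnyDamage and routes hits into ProcessDamage.
; ProcessDamage only prints the incoming damage and returns a zeroed applied/reduced/absorbed struct.
; A client-named ShowDamage event prints applied damage, but its call is not wired into execution.
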(event `self.ReceiveBeginPlay`
  ;[1 1 1] Begin Play
  ;[1 1 1] Bind On Any Damage Event
  (add `Actor.OnTakeAnyDamage` (`self.GetOwner`) (`|CreateDelegate` :!event `On Any Damage`)))

(event `On Any Damage`
  (params (DamagedActor :type "Actor Object Reference") (Damage :type "Float (double-precision)") (DamageType :type "DamageType Object Reference") (InstigatedBy :type "Controller Object Reference") (DamageCauser :type "Actor Object Reference"))
  (bind _return (`self.Process Damage` Damage InstigatedBy DamageCauser DamageType)))

(event `CLIENT // Show Damage`
  (params (`Damage Info` :type "/Game/SYN/DamageSystem/Structures/S_DamageReturnInfo Structure (by ref)"))
  (`KismetSystemLibrary.PrintString` (`KismetStringLibrary.Concat_StrStr` "Local // Damage " (`KismetStringLibrary.Conv_DoubleToString` (`.AppliedDamage_3_A08171B54CB5C9DC4DF728A4A165ACC6` (break `/Game/SYN/DamageSystem/Structures/S_DamageReturnInfo` `Damage Info`))))))

(fn `Process Damage`
  (params (`Base Damage` :type "Float (double-precision)") (`Investigated by` :type "Controller Object Reference") (`Damage Causer` :type "Actor Object Reference") (`Damage Type` :type "DamageType Object Reference"))
  (returns (Return :type "/Game/SYN/DamageSystem/Structures/S_DamageReturnInfo Structure"))
  (`KismetSystemLibrary.PrintString` (`KismetStringLibrary.Concat_StrStr` (`KismetSystemLibrary.GetDisplayName` (`self.GetOwner`)) " taking " (`KismetStringLibrary.Conv_DoubleToString` `Base Damage`) "damage") true true (struct :`R` 1.0 :`B` 0.156425 :`A` 1.0) 10.0)
  (return (make `/Game/SYN/DamageSystem/Structures/S_DamageReturnInfo` 0.0)))